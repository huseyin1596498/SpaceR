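; Flyable Ship that also signals when the third-person character enters or leaves its interior and cockpit.
; Mouse wheel changes a persistent throttle, W/S and A/D accumulate pitch and roll rates, and the mouse rotates the camera.
; Tick applies per-frame offsets without delta-time scaling, moving the first Ship found and its child actor but rotating itself.
; Two trigger volumes fire the enter and exit dispatchers.
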(event OnComponentBeginOverlap(Pilotrigger)
  (params (OverlappedComponent :type Primitive%20Component%20Object%20Reference) (OtherActor :type Actor%20Object%20Reference) (OtherComp :type Primitive%20Component%20Object%20Reference) (OtherBodyIndex :type Integer) (bFromSweep :type Boolean) (SweepResult :type Hit%20Result%20Structure%20%28by%20ref%29))
  (bind _outactors (Actor|GetAllActorsOfClass "/Game/Blueprints/Charachters/ThirdPersonCharacter.ThirdPersonCharacter_C"))
  (if (== OtherActor (Utilities|Array|Get(acopy) _outactors))
    (Default|CallCockpitEnter)))

(event OnComponentEndOverlap(Pilotrigger)
  (params (OverlappedComponent :type Primitive%20Component%20Object%20Reference) (OtherActor :type Actor%20Object%20Reference) (OtherComp :type Primitive%20Component%20Object%20Reference) (OtherBodyIndex :type Integer))
  (bind _outactors (Actor|GetAllActorsOfClass "/Game/Blueprints/Charachters/ThirdPersonCharacter.ThirdPersonCharacter_C"))
  (if (== OtherActor (Utilities|Array|Get(acopy) _outactors))
    (Default|CallCockpitExit)))

(event OnComponentBeginOverlap(ShipTrigger)
  (params (OverlappedComponent :type Primitive%20Component%20Object%20Reference) (OtherActor :type Actor%20Object%20Reference) (OtherComp :type Primitive%20Component%20Object%20Reference) (OtherBodyIndex :type Integer) (bFromSweep :type Boolean) (SweepResult :type Hit%20Result%20Structure%20%28by%20ref%29))
  (bind _outactors (Actor|GetAllActorsOfClass "/Game/Blueprints/Charachters/ThirdPersonCharacter.ThirdPersonCharacter_C"))
  (if (== OtherActor (Utilities|Array|Get(acopy) _outactors))
    (Default|CallInsideShipE)))

(event OnComponentActivated(ShipTrigger)
  (params (Component :type Actor%20Component%20Object%20Reference) (bReset :type Boolean)))

(event OnComponentEndOverlap(ShipTrigger)
  (params (OverlappedComponent :type Primitive%20Component%20Object%20Reference) (OtherActor :type Actor%20Object%20Reference) (OtherComp :type Primitive%20Component%20Object%20Reference) (OtherBodyIndex :type Integer))
  (bind _outactors (Actor|GetAllActorsOfClass "/Game/Blueprints/Charachters/ThirdPersonCharacter.ThirdPersonCharacter_C"))
  (if (== OtherActor (Utilities|Array|Get(acopy) _outactors))
    (Default|CallOutsideShip)))

(event EventBeginPlay)

(event EventTick
  (params (DeltaSeconds :type Float%20%28single-precision%29))
  (Utilities|FlowControl|Sequence
    (:then_0
      (if (Variables|Default|GetGass)
        (Variables|Default|SetFowardPush (+ (Variables|Default|GetFowardPush) 1.0))))
    (:then_1
      (if (Variables|Default|GetLessGassB)
        (Variables|Default|SetFowardPush (- (Variables|Default|GetFowardPush) 1.0))))
    (:then_2
      (bind _outactors (Actor|GetAllActorsOfClass "Ship_C"))
      (Transformation|SetActorLocation (Utilities|Array|Get(acopy) _outactors) (+ (Transformation|GetActorLocation (Utilities|Array|Get(acopy) _outactors)) (* (Transformation|GetActorForwardVector (Utilities|Array|Get(acopy) _outactors)) (Variables|Default|GetFowardPush))) false false)
      (Transformation|SetWorldLocation (Variables|Ship_C|GetChildActor (Utilities|Array|Get(acopy) _outactors)) (+ (Transformation|GetActorLocation) (* (Transformation|GetActorForwardVector) 3e+01)) false false))
    (:then_3
      (if (Variables|Default|GetLook%20up)
        (Variables|Default|SetLookUpF (+ (Variables|Default|GetLookUpF) -0.0005))))
    (:then_4
      (if (Variables|Default|GetLoopDown)
        (Variables|Default|SetLookUpF (+ (Variables|Default|GetLookUpF) 0.0005))))
    (:then_5
      (Transformation|AddActorLocalRotation (Math|Rotator|MakeRotator 0.0 (* (/ (Utilities|Time|GetGameTimeinSeconds) (Utilities|Time|GetGameTimeinSeconds)) (Variables|Default|GetLookUpF)) 0.0) false false))
    (:then_9
      (if (Variables|Default|GetLook%20Left)
        (Variables|Default|SetLookLeft/Right (+ (Variables|Default|GetLookLeft/Right) 0.0005))))
    (:then_10
      (if (Variables|Default|GetLookRight)
        (Variables|Default|SetLookLeft/Right (+ (Variables|Default|GetLookLeft/Right) -0.0005))))
    (:then_11
      (Transformation|AddActorLocalRotation (Math|Rotator|MakeRotator (* (/ (Utilities|Time|GetGameTimeinSeconds) (Utilities|Time|GetGameTimeinSeconds)) (Variables|Default|GetLookLeft/Right)) 0.0 0.0) false false))))

(event Input|MouseEvents|MouseX
  (params (AxisValue :type Float%20%28single-precision%29))
  (Transformation|AddLocalRotation (Variables|Default|GetCamera) (Math|Rotator|MakeRotator 0.0 0.0 (* (/ (Utilities|Time|GetGameTimeinSeconds) (Utilities|Time|GetGameTimeinSeconds)) AxisValue)) false false))

(event Input|MouseEvents|MouseY
  (params (AxisValue :type Float%20%28single-precision%29))
  (Transformation|AddLocalRotation (Variables|Default|GetCamera) (Math|Rotator|MakeRotator 0.0 (* (/ (Utilities|Time|GetGameTimeinSeconds) (Utilities|Time|GetGameTimeinSeconds)) AxisValue) 0.0) false false))

(event Input|MouseEvents|MouseWheelAxis
  (params (AxisValue :type Float%20%28single-precision%29))
  (if (> AxisValue 0.0)
    (Variables|Default|SetGass true)
    (elif (< AxisValue 0.0)
      (Variables|Default|SetLessGassB true)
      (elif (== AxisValue 0.0)
        (Variables|Default|SetGass false)
        (Variables|Default|SetLessGassB false)))))

(event Input|KeyboardEvents|S
  (params (Key :type Key%20Structure))
  (:Pressed
    (Variables|Default|SetLoopDown true))
  (:Released
    (Variables|Default|SetLoopDown false)))

(event Input|KeyboardEvents|D
  (params (Key :type Key%20Structure))
  (:Pressed
    (Variables|Default|SetLookRight true))
  (:Released
    (Variables|Default|SetLookRight false)))

(event Input|KeyboardEvents|A
  (params (Key :type Key%20Structure))
  (:Pressed
    (Variables|Default|SetLook%20Left true))
  (:Released
    (Variables|Default|SetLook%20Left false)))

(event Input|KeyboardEvents|W
  (params (Key :type Key%20Structure))
  (:Pressed
    (Variables|Default|SetLook%20up true))
  (:Released
    (Variables|Default|SetLook%20up false)))

(fn ConstructionScript)

(fn NewFunction0)