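; An interactive radio actor that the player toggles on and off while standing inside its trigger box.
; Box overlaps with the first ThirdPersonCharacter set PlayerInside, which gates that character's PlayRadio event, re-bound here every Tick.
; A FlipFlop alternates between fading in two static layers followed by a delayed station song, and staggered fade-outs that leave one static layer lingering before it stops.
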(event OnComponentBeginOverlap(Box)
  (params (OverlappedComponent :type Primitive%20Component%20Object%20Reference) (OtherActor :type Actor%20Object%20Reference) (OtherComp :type Primitive%20Component%20Object%20Reference) (OtherBodyIndex :type Integer) (bFromSweep :type Boolean) (SweepResult :type Hit%20Result%20Structure%20%28by%20ref%29))
  (bind _outactors (Actor|GetAllActorsOfClass "/Game/Blueprints/Charachters/ThirdPersonCharacter.ThirdPersonCharacter_C"))
  (if (== (Utilities|Array|Get(acopy) _outactors) OtherActor)
    (Variables|Default|SetPlayerInside? true)))

(event OnComponentEndOverlap(Box)
  (params (OverlappedComponent :type Primitive%20Component%20Object%20Reference) (OtherActor :type Actor%20Object%20Reference) (OtherComp :type Primitive%20Component%20Object%20Reference) (OtherBodyIndex :type Integer))
  (bind _outactors (Actor|GetAllActorsOfClass "/Game/Blueprints/Charachters/ThirdPersonCharacter.ThirdPersonCharacter_C"))
  (if (== (Utilities|Array|Get(acopy) _outactors) OtherActor)
    (Variables|Default|SetPlayerInside? false)))

(event Custom|CustomEvent_0
  (if (Variables|Default|GetPlayerInside?)
    (Utilities|FlowControl|FlipFlop
      (:A
        (Development|PrintString "on")
        (Audio|Components|Audio|FadeIn (Variables|Default|GetStatic1) 1.0 1.0 0.0 :!class /Script/Engine.AudioComponent)
        (Audio|Components|Audio|FadeIn (Variables|Default|GetStatic2) 1.0 1.0 0.0 :!class /Script/Engine.AudioComponent)
        (Utilities|FlowControl|Delay 0.5)
        (Audio|Components|Audio|FadeIn (Variables|Default|GetStation1Song1) 1.0 1.0 0.0 :!class /Script/Engine.AudioComponent))
      (:B
        (Development|PrintString "off")
        (Audio|Components|Audio|FadeOut (Variables|Default|GetStation1Song1) 0.2 0.0 :!class /Script/Engine.AudioComponent)
        (Audio|Components|Audio|FadeOut (Variables|Default|GetStatic2) 0.4 0.0 :!class /Script/Engine.AudioComponent)
        (Utilities|FlowControl|Delay 5.0)
        (Audio|Components|Audio|FadeOut (Variables|Default|GetStatic1) 0.1 0.0 :!class /Script/Engine.AudioComponent)))))

(event EventTick
  (params (DeltaSeconds :type Float%20%28single-precision%29))
  (bind _outactors (Actor|GetAllActorsOfClass "/Game/Blueprints/Charachters/ThirdPersonCharacter.ThirdPersonCharacter_C"))
  (EventDispatchers|BindEventtoPlayRadio (Utilities|Array|Get(acopy) _outactors) (delegate Custom|CustomEvent_0)))

(event EventBeginPlay
  (Audio|Components|Audio|FadeOut (Variables|Default|GetStatic1) 0.0 0.0 :!class /Script/Engine.AudioComponent))

(fn ConstructionScript)