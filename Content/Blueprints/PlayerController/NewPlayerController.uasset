(event Custom|CustomEvent_1
  (Variables|Default|SetInsdie%20Cockpit false))

(event Custom|CustomEvent_0
  (Variables|Default|SetInsdie%20Cockpit true))

(event Custom|CustomEvent_2
  (Variables|Default|SetInsideTurret true))

(event EventTick
  (params (DeltaSeconds :type Float%20%28single-precision%29))
  (Utilities|FlowControl|Sequence
    (:then_0
      (bind _outactors (Actor|GetAllActorsOfClass "/Game/Blueprints/Ships/Ship.Ship_C"))
      (EventDispatchers|BindEventtoCockpitExit _outactors (delegate Custom|CustomEvent_1)))
    (:then_1
      (bind _outactors_2 (Actor|GetAllActorsOfClass "/Game/Blueprints/Ships/Ship.Ship_C"))
      (EventDispatchers|BindEventtoCockpitEnter _outactors_2 (delegate Custom|CustomEvent_0)))
    (:then_2
      (bind _outactors_3 (Actor|GetAllActorsOfClass "/Game/Blueprints/Turret/Turret.Turret_C"))
      (EventDispatchers|BindEventtoInsideTurret _outactors_3 (delegate Custom|CustomEvent_2)))))

(event EventBeginPlay
  (bind _returnvalue (UserInterface|CreateWidget "/Game/UI/MouseCursor.MouseCursor_C"))
  (Class|PlayerController|SetMouseCursorWidget (Game|GetPlayerController 0) "Default" _returnvalue))

(event Input|KeyboardEvents|4
  (params (Key :type Key%20Structure))
  (:Pressed
    (bind _outactors (Actor|GetAllActorsOfClass 0))
    (Pawn|Possess)))

(event Input|KeyboardEvents|3
  (params (Key :type Key%20Structure))
  (:Pressed
    (bind _outactors (Actor|GetAllActorsOfClass "/Game/Blueprints/Charachters/ThirdPersonCharacter.ThirdPersonCharacter_C"))
    (Variables|/Script/Engine.Pawn|SetAIControllerClass (Utilities|Array|Get(acopy) _outactors) "NewPlayerController_C")
    (bind _outactors_2 (Actor|GetAllActorsOfClass "/Game/Blueprints/Ships/Ship.Ship_C"))
    (Variables|/Script/Engine.Pawn|SetAIControllerClass (Utilities|Array|Get(acopy) _outactors_2) "/Script/AIModule.AIController")
    (bind _outactors_3 (Actor|GetAllActorsOfClass "/Game/Blueprints/Turret/Turret.Turret_C"))
    (Variables|/Script/Engine.Pawn|SetAIControllerClass (Utilities|Array|Get(acopy) _outactors_3) "/Script/AIModule.AIController")
    (Transformation|DetachFromActor (Utilities|Array|Get(acopy) _outactors) "KeepWorld" "KeepWorld" "KeepWorld")
    (bind _outactors_4 (Actor|GetAllActorsOfClass "/Game/Blueprints/Charachters/ThirdPersonCharacter.ThirdPersonCharacter_C"))
    (Pawn|Possess (Utilities|Array|Get(acopy) _outactors_4))
    (Utilities|FlowControl|Sequence
      (:then_0
        (Utilities|FlowControl|DoOnce false) ; enters at Reset
      )
      (:then_1
        (Utilities|FlowControl|DoOnce false) ; enters at Reset
      ))))

(event Input|KeyboardEvents|5
  (params (Key :type Key%20Structure)))

(event Input|KeyboardEvents|I
  (params (Key :type Key%20Structure))
  (:Pressed
    (if (Variables|Default|GetInsdie%20Cockpit)
      (Utilities|FlowControl|DoOnce false
        (:Completed
          (bind _outactors (Actor|GetAllActorsOfClass "/Game/Blueprints/Ships/Ship.Ship_C"))
          (Pawn|Possess (Utilities|Array|Get(acopy) _outactors))
          (Default|CallStartengine)
          (bind _outactors_2 (Actor|GetAllActorsOfClass "/Game/Blueprints/Charachters/ThirdPersonCharacter.ThirdPersonCharacter_C"))
          (Variables|/Script/Engine.Pawn|SetAIControllerClass (Utilities|Array|Get(acopy) _outactors_2) "/Script/AIModule.AIController")
          (bind _outactors_3 (Actor|GetAllActorsOfClass "/Game/Blueprints/Ships/Ship.Ship_C"))
          (Variables|/Script/Engine.Pawn|SetAIControllerClass (Utilities|Array|Get(acopy) _outactors_3) "NewPlayerController_C")
          (Transformation|AttachActorToActor (Utilities|Array|Get(acopy) _outactors_2) (Utilities|Array|Get(acopy) _outactors_3) "None" "KeepWorld" "KeepWorld" "KeepWorld" true)))
      (elif (Variables|Default|GetInsideTurret)
        (Utilities|FlowControl|DoOnce false
          (:Completed
            (bind _outactors_4 (Actor|GetAllActorsOfClass "/Game/Blueprints/Turret/Turret.Turret_C"))
            (Pawn|Possess (Utilities|Array|Get(acopy) _outactors_4))
            (bind _outactors_5 (Actor|GetAllActorsOfClass "/Game/Blueprints/Charachters/ThirdPersonCharacter.ThirdPersonCharacter_C"))
            (Variables|/Script/Engine.Pawn|SetAIControllerClass (Utilities|Array|Get(acopy) _outactors_5) "/Script/AIModule.AIController")
            (bind _outactors_6 (Actor|GetAllActorsOfClass "/Game/Blueprints/Turret/Turret.Turret_C"))
            (Variables|/Script/Engine.Pawn|SetAIControllerClass (Utilities|Array|Get(acopy) _outactors_6) "NewPlayerController_C")
            (Transformation|AttachActorToActor (Utilities|Array|Get(acopy) _outactors_5) 0 "None" "KeepWorld" "KeepWorld" "KeepWorld" true)))))))

(fn ConstructionScript)