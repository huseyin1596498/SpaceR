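; Turret bullet actor that flies in a straight line and destroys itself one second after spawning.
; Tick moves the Sphere component a fixed distance along its negative forward vector, without sweep and without scaling by delta time, so speed depends on frame rate.
; It has no hit or damage logic, as the overlap event is an unused, disabled stub.
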(event EventBeginPlay
  (Utilities|FlowControl|Delay 1.0)
  (Actor|DestroyActor))

(event Collision|EventActorBeginOverlap
  (params (OtherActor :type Actor%20Object%20Reference)))

(event EventTick
  (params (DeltaSeconds :type Float%20%28single-precision%29))
  (Transformation|SetWorldLocation (Variables|Default|GetSphere) (+ (Transformation|GetWorldLocation (Variables|Default|GetSphere)) (* (Math|Vector|GetForwardVector (Variables|Default|GetSphere)) -1e+03)) false false))

(fn ConstructionScript)