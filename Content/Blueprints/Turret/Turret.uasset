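; Turret actor that aims with the mouse and fires bullets on left click.
; Mouse axes add local yaw and inverted pitch to the root, Tick zeroes roll, and clicks spawn scaled Bullet actors at the Bullet component's transform.
; A box overlap fires InsideTurret and OutsideTurret dispatchers when the first ThirdPersonCharacter enters or leaves.
; Nothing in this graph gates input on that overlap, and the game-time division in aiming cancels itself out.
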(event OnComponentBeginOverlap(Box)
  (params (OverlappedComponent :type Primitive%20Component%20Object%20Reference) (OtherActor :type Actor%20Object%20Reference) (OtherComp :type Primitive%20Component%20Object%20Reference) (OtherBodyIndex :type Integer) (bFromSweep :type Boolean) (SweepResult :type Hit%20Result%20Structure%20%28by%20ref%29))
  (bind _outactors (Actor|GetAllActorsOfClass "/Game/Blueprints/Charachters/ThirdPersonCharacter.ThirdPersonCharacter_C"))
  (if (== (Utilities|Array|Get(acopy) _outactors) OtherActor)
    (Default|CallInsideTurret)))

(event OnComponentEndOverlap(Box)
  (params (OverlappedComponent :type Primitive%20Component%20Object%20Reference) (OtherActor :type Actor%20Object%20Reference) (OtherComp :type Primitive%20Component%20Object%20Reference) (OtherBodyIndex :type Integer))
  (bind _outactors (Actor|GetAllActorsOfClass "/Game/Blueprints/Charachters/ThirdPersonCharacter.ThirdPersonCharacter_C"))
  (if (== (Utilities|Array|Get(acopy) _outactors) OtherActor)
    (Default|CallOutsideTurret)))

(event EventTick
  (params (DeltaSeconds :type Float%20%28single-precision%29))
  (bind _defaultsceneroot (Variables|Default|GetDefaultSceneRoot))
  (bind _returnvalue (Transformation|GetWorldRotation _defaultsceneroot))
  (Transformation|SetWorldRotation _defaultsceneroot (Math|Rotator|MakeRotator 0.0 (.pitch _returnvalue) (.yaw _returnvalue)) false false))

(event Input|MouseEvents|MouseX
  (params (AxisValue :type Float%20%28single-precision%29))
  (Transformation|AddLocalRotation (Variables|Default|GetDefaultSceneRoot) (Math|Rotator|MakeRotator 0.0 0.0 (* (/ (Utilities|Time|GetGameTimeinSeconds) (Utilities|Time|GetGameTimeinSeconds)) AxisValue)) false false))

(event Input|MouseEvents|MouseY
  (params (AxisValue :type Float%20%28single-precision%29))
  (Transformation|AddLocalRotation (Variables|Default|GetDefaultSceneRoot) (Math|Rotator|MakeRotator 0.0 (* (* (/ (Utilities|Time|GetGameTimeinSeconds) (Utilities|Time|GetGameTimeinSeconds)) AxisValue) -1.0) 0.0) false false))

(event Input|MouseEvents|LeftMouseButton
  (params (Key :type Key%20Structure))
  (bind _bullet (Variables|Default|Getbullet))
  (bind _returnvalue (Transformation|GetWorldTransform _bullet))
  (:Pressed
    (Game|SpawnActorfromClass "/Game/Blueprints/Turret/bullet.bullet_C" (Math|Transform|MakeTransform (.location _returnvalue) (.rotation _returnvalue) "0.300000,0.300000,1.000000") "Undefined" 0 0)))

(fn ConstructionScript)